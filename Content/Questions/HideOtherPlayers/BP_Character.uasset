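; Player character Blueprint that toggles whether player meshes are visible to anyone other than their owners, using the H key.
; H flips a local hidden flag and passes it to a server event, which loops over player controllers under authority.
; Each controlled BP_Character then runs a multicast that sets Only Owner See on its mesh, so the toggle applies to all players rather than only the requester.
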(event Custom|ServerCalled_HideOtherPlayers
  (params (Hide :type Boolean))
  (Networking|SwitchHasAuthority
    (:Authority
      (bind _returnvalue (Class|GameModeBase|GetNumPlayers (Game|GetGameMode)))
      (for _index (range 0 (- _returnvalue 1))
        (bind _asbp_character (Utilities|Casting|CastToBP_Character (Pawn|GetControlledPawn (Game|GetPlayerController _index))))
        (CallFunction|MulticastHideOtherPlayers _asbp_character Hide)))))

(event Custom|Multicast_HideOtherPlayers
  (params (Hide :type Boolean))
  (Rendering|SetOnlyOwnerSee (Variables|Character|GetMesh) Hide :!class /Script/Engine.PrimitiveComponent))

(event EventBeginPlay)

(event Collision|EventActorBeginOverlap
  (params (OtherActor :type Actor%20Object%20Reference)))

(event EventTick
  (params (DeltaSeconds :type Float%20%28single-precision%29)))

(event Input|KeyboardEvents|H
  (params (Key :type Key%20Structure))
  (:Pressed
    (bind _output_get (Variables|Default|SetCurrentlyHidden (not (Variables|Default|GetCurrentlyHidden))))
    (CallFunction|ServerCalledHideOtherPlayers _output_get)))

(fn ConstructionScript)