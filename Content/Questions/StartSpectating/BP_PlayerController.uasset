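; Player controller Blueprint that tests switching the player between spectating and playing through debug keys.
; K and L call StartSpectating and StartPlaying, which are not defined in this graph, and matching Trigger events wrap the same calls.
; N and M use variants that store the controlled pawn in OldPawn before spectating and possess it again after resuming play.
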(event Custom|Trigger_StartSpectatingAndStoreOldActor
  (Variables|Default|SetOldPawn (Pawn|GetControlledPawn self))
  (Class|StartSpectatingPlayerController|StartSpectating))

(event Custom|Trigger_StartPlayingAndPossessOldActor
  (Class|StartSpectatingPlayerController|StartPlaying)
  (Pawn|Possess (Variables|Default|GetOldPawn)))

(event Custom|Trigger_StartSpectating
  (Class|StartSpectatingPlayerController|StartSpectating))

(event Custom|Trigger_StartPlaying
  (Class|StartSpectatingPlayerController|StartPlaying))

(event EventBeginPlay)

(event EventTick
  (params (DeltaSeconds :type Float%20%28single-precision%29)))

(event Input|KeyboardEvents|M
  (params (Key :type Key%20Structure))
  (:Pressed
    (CallFunction|TriggerStartPlayingandPossessOldActor)))

(event Input|KeyboardEvents|N
  (params (Key :type Key%20Structure))
  (:Pressed
    (CallFunction|TriggerStartSpectatingandStoreOldActor)))

(event Input|KeyboardEvents|K
  (params (Key :type Key%20Structure))
  (:Pressed
    (Class|StartSpectatingPlayerController|StartSpectating)))

(event Input|KeyboardEvents|L
  (params (Key :type Key%20Structure))
  (:Pressed
    (Class|StartSpectatingPlayerController|StartPlaying)))

(fn ConstructionScript)